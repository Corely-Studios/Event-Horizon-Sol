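; BP_Interactable_Master is, by its name, the base interactable, an item the player picks up and holds.
; Interact drops the player's current item, spawns a same-class clone without physics or collision, attaches it to the hand socket and destroys the original.
; The clone becomes the held item, initializes its UI if throwable and is messaged to arm its sound.
; An armed item plays an impact sound once upon hitting a Floor-tagged actor.
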(event `/Game/BPs/Interactable/Interface/BPI_Interaction.Interact`
  (params (`Player Ref` :type "/Game/BPs/Characters/FirstPersonBP/Blueprints/FirstPersonCharacter Object Reference") (`Clicked Component` :type "PrimitiveComponent Object Reference"))
  (`/Game/BPs/Characters/FirstPersonBP/Blueprints/FirstPersonCharacter.Drop Item` `Player Ref`)
  (bind _returnvalue (`|SpawnActorFromClass` (`GameplayStatics.GetObjectClass` self) (`self.GetTransform` self) "Undefined" "OverrideRootScale" null null))
  (bind _returnvalue_2 (`self.GetComponentByClass` _returnvalue "/Script/Engine.StaticMeshComponent"))
  (`PrimitiveComponent.SetSimulatePhysics` _returnvalue_2 false)
  (`PrimitiveComponent.SetCollisionEnabled` _returnvalue_2 "NoCollision")
  (`self.K2_AttachToComponent` _returnvalue (`/Game/BPs/Characters/FirstPersonBP/Blueprints/FirstPersonCharacter.Hand Socket` `Player Ref`) "Hand Socket" "SnapToTarget" "SnapToTarget" "KeepWorld" true)
  (set `/Game/BPs/Characters/FirstPersonBP/Blueprints/FirstPersonCharacter.Current Held Item` _returnvalue `Player Ref`)
  (`self.K2_DestroyActor`)
  (`|ExecutionSequence`
    (:`then_0`
      (bind _asbp_throwable (cast `/Game/BPs/Interactable/Throwable/BP_Throwable` _returnvalue))
      (`/Game/BPs/Interactable/Throwable/BP_Throwable.Initialize UI` _asbp_throwable))
    (:`then_1`
      (message `/Game/BPs/Interactable/Interface/BPI_SoundControl.Trigger Clone Sound` _returnvalue))))

(event `/Game/BPs/Interactable/Interface/BPI_SoundControl.Trigger Clone Sound`
  (set `self.Can_PlaySound?` true))

(event `self.Object.OnComponentHit`
  (params (HitComponent :type "PrimitiveComponent Object Reference") (OtherActor :type "Actor Object Reference") (OtherComp :type "PrimitiveComponent Object Reference") (NormalImpulse :type "Vector Structure") (Hit :type "HitResult Structure (by ref)"))
  (if (`self.ActorHasTag` OtherActor "Floor")
    (if (`self.Can_PlaySound?`)
      (`GameplayStatics.PlaySoundAtLocation` (`self.Impact Sound`) (`self.K2_GetActorLocation`) (struct) 1.0 1.0 0.0 null null null)
      (set `self.Can_PlaySound?` false))))

(fn `Record Death`
  (returns (`Current Deaths` :type Integer))
  (return 0))

(fn `UserConstructionScript`)