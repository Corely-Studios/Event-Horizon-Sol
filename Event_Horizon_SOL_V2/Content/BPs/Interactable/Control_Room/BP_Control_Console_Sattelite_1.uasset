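; Interactable control console in the Sattelite_01 level that teleports the player back to Game_Map.
; A sphere overlap shows and hides four widgets while the player is in range.
; Interact reads the clicked button's tag, then a shared DoOnce plays a timeline that pushes the button in.
; All four buttons then trigger the same player level-streaming teleport, and the DoOnce resets after a short delay.
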(event `self.Sphere.OnComponentBeginOverlap`
  (params (OverlappedComponent :type "PrimitiveComponent Object Reference") (OtherActor :type "Actor Object Reference") (OtherComp :type "PrimitiveComponent Object Reference") (OtherBodyIndex :type Integer) (bFromSweep :type Boolean) (SweepResult :type "HitResult Structure (by ref)"))
  (if (`self.ActorHasTag` OtherActor "Player")
    (`SceneComponent.SetVisibility` (`self.Widget`) true false)
    (`SceneComponent.SetVisibility` (`self.Widget1`) true false)
    (`SceneComponent.SetVisibility` (`self.Widget2`) true false)
    (`SceneComponent.SetVisibility` (`self.Widget3`) true false)))

(event `self.Sphere.OnComponentEndOverlap`
  (params (OverlappedComponent :type "PrimitiveComponent Object Reference") (OtherActor :type "Actor Object Reference") (OtherComp :type "PrimitiveComponent Object Reference") (OtherBodyIndex :type Integer))
  (if (`self.ActorHasTag` OtherActor "Player")
    (`SceneComponent.SetVisibility` (`self.Widget`) false false)
    (`SceneComponent.SetVisibility` (`self.Widget1`) false false)
    (`SceneComponent.SetVisibility` (`self.Widget2`) false false)
    (`SceneComponent.SetVisibility` (`self.Widget3`) false false)))

(event `/Game/BPs/Interactable/Interface/BPI_Interaction.Interact`
  (params (`Player Ref` :type "/Game/BPs/Characters/FirstPersonBP/Blueprints/FirstPersonCharacter Object Reference") (`Clicked Component` :type "PrimitiveComponent Object Reference"))
  (bind _player (`self.Player`))
  (bind _starting_position (`self.Starting Position`))
  (set `self.Clicked Object Ref` `Clicked Component`)
  (set `self.Player` `Player Ref`)
  (switch `name` (`|GetArrayItem` (`ActorComponent.ComponentTags` (`self.Clicked Object Ref`)))
    (:`Button1`
      _)
    (:`Button2`
      _)
    (:`Button3`
      _)
    (:`Button4`
      _))
  (`/Engine/EditorBlueprintResources/StandardMacros.DoOnce` false :!label _label
    (:`Completed`
      (set `self.Starting Position` (`SceneComponent.RelativeLocation` (`self.Clicked Object Ref`)))
      (bind (_direction _alpha) (`Timeline|Button TM` :!via `PlayFromStart`)
        (:`Update`
          (`SceneComponent.K2_SetRelativeLocation` (`self.Clicked Object Ref`) (`KismetMathLibrary.VLerp` _starting_position (+ (0.0 -2.0 0.0) _starting_position) _alpha) false false))
        (:`Finished`
          (switch `name` (`|GetArrayItem` (`ActorComponent.ComponentTags` (`self.Clicked Object Ref`)))
            (:`Button1`
              (`/Game/BPs/Characters/FirstPersonBP/Blueprints/FirstPersonCharacter.Level Streaming Teleportation event` _player "Game_Map" "Sattelite_01" (-1220.180664 -638.247253 226.284607)))
            (:`Button2`
              (`/Game/BPs/Characters/FirstPersonBP/Blueprints/FirstPersonCharacter.Level Streaming Teleportation event` _player "Game_Map" "Sattelite_01" (-1220.180664 -638.247253 226.284607)))
            (:`Button3`
              (`/Game/BPs/Characters/FirstPersonBP/Blueprints/FirstPersonCharacter.Level Streaming Teleportation event` _player "Game_Map" "Sattelite_01" (-1220.180664 -638.247253 226.284607)))
            (:`Button4`
              (`/Game/BPs/Characters/FirstPersonBP/Blueprints/FirstPersonCharacter.Level Streaming Teleportation event` _player "Game_Map" "Sattelite_01" (-1220.180664 -638.247253 226.284607))))
          (`KismetSystemLibrary.Delay` 1.5)
          (goto _label :!via `Reset`))))))

(fn `Record Death`
  (returns (`Current Deaths` :type Integer))
  (return 0))

(fn `UserConstructionScript`)