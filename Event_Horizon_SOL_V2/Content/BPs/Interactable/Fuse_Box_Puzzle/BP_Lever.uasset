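; BP_Lever is the interactable lever of the fuse box puzzle, showing a prompt widget while the player is inside its sphere.
; Interact swings the hinge with a timeline and reverses it after a delay.
; When the timeline finishes, a socketed fuse triggers a console message and electric sound.
; Without a fuse, a DoOnce-guarded WBP_Lever popup appears briefly.
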(event `self.Sphere.OnComponentBeginOverlap`
  (params (OverlappedComponent :type "PrimitiveComponent Object Reference") (OtherActor :type "Actor Object Reference") (OtherComp :type "PrimitiveComponent Object Reference") (OtherBodyIndex :type Integer) (bFromSweep :type Boolean) (SweepResult :type "HitResult Structure (by ref)"))
  (if (`self.ActorHasTag` OtherActor "Player")
    (`SceneComponent.SetVisibility` (`self.Widget`) true false)))

(event `self.Sphere.OnComponentEndOverlap`
  (params (OverlappedComponent :type "PrimitiveComponent Object Reference") (OtherActor :type "Actor Object Reference") (OtherComp :type "PrimitiveComponent Object Reference") (OtherBodyIndex :type Integer))
  (if (`self.ActorHasTag` OtherActor "Player")
    (`SceneComponent.SetVisibility` (`self.Widget`) false false)))

(event `/Game/BPs/Interactable/Interface/BPI_Interaction.Interact`
  (params (`Player Ref` :type "/Game/BPs/Characters/FirstPersonBP/Blueprints/FirstPersonCharacter Object Reference") (`Clicked Component` :type "PrimitiveComponent Object Reference"))
  (set `self.Player` `Player Ref`)
  (if (not (not (`self.Socket Have Fuse?`)))
    (`/Engine/EditorBlueprintResources/StandardMacros.DoOnce` false
      (:`Completed`
        _)))
  (`|ExecutionSequence`
    (:`then_0`
      (bind (_direction _alpha) (`Timeline|Lever TM` :!label _label)
        (:`Update`
          (`SceneComponent.K2_SetRelativeRotation` (`self.Hinge`) (`KismetMathLibrary.RLerp` (struct) (struct :`Roll` 180.0) _alpha) false false))
        (:`Finished`
          (if (`self.Socket Have Fuse?`)
            (message `/Game/BPs/Interactable/Interface/BPI_Interaction.Socket Have Fuse` (`self.Console_Ref`))
            (`GameplayStatics.PlaySoundAtLocation` "/Game/BPs/Interactable/Fuse_Box_Puzzle/Lever_Sound/electric_sound.electric_sound" (`self.K2_GetActorLocation`) (struct) 1.0 1.0 0.0 null null null)
            (else
              (`/Engine/EditorBlueprintResources/StandardMacros.DoOnce` false :!label _label_2
                (:`Completed`
                  (bind _returnvalue (`|CreateWidget` "/Game/UI/Widgets/Puzzles/Fuse_Box_Puzzle/WBP_Lever.WBP_Lever_C"))
                  (`UserWidget.AddToViewport` _returnvalue 0)
                  (`KismetSystemLibrary.Delay` 2.0)
                  (`Widget.RemoveFromParent` _returnvalue)
                  (goto _label_2 :!via `Reset`))))))))
    (:`then_1`
      (`KismetSystemLibrary.Delay` 1.5)
      (goto _label :!via `Reverse`))))

(event `/Game/BPs/Interactable/Interface/BPI_Interaction.Socket Have Fuse`
  (set `self.Socket Have Fuse?` true))

(fn `Record Death`
  (returns (`Current Deaths` :type Integer))
  (return 0))

(fn `UserConstructionScript`)