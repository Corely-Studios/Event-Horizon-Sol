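; Fuse box puzzle interactable that accepts a fuse carried by the player and notifies a linked lever.
; On Interact, it checks that the held item's class is exactly BP_Fuse, then destroys it and clears the player's held reference.
; It reveals the PhantomFuse component to show the inserted fuse and calls SocketHaveFuseMessage on TargetedLever.
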(event `/Game/BPs/Interactable/Interface/BPI_Interaction.Interact`
  (params (`Player Ref` :type "/Game/BPs/Characters/FirstPersonBP/Blueprints/FirstPersonCharacter Object Reference") (`Clicked Component` :type "PrimitiveComponent Object Reference"))
  (bind _current_held_item (`/Game/BPs/Characters/FirstPersonBP/Blueprints/FirstPersonCharacter.Current Held Item` `Player Ref`))
  (if (== (`GameplayStatics.GetObjectClass` _current_held_item) "/Game/BPs/Interactable/Fuse_Box_Puzzle/BP_Fuse.BP_Fuse_C")
    (`self.K2_DestroyActor` _current_held_item)
    (set `/Game/BPs/Characters/FirstPersonBP/Blueprints/FirstPersonCharacter.Current Held Item` null `Player Ref`)
    (`SceneComponent.SetVisibility` (`self.Phantom Fuse`) true false)
    (message `/Game/BPs/Interactable/Interface/BPI_Interaction.Socket Have Fuse` (`self.Targeted Lever`))))

(fn `Record Death`
  (returns (`Current Deaths` :type Integer))
  (return 0))

(fn `UserConstructionScript`)