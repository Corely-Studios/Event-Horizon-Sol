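; BP_Automatic_Door is an automatic sliding double door that opens for actors tagged Player or AI.
; Box overlap begin plays OpenCloseTimeline, whose alpha lerps Door1 and Door2 apart along relative Y without sweeping.
; End overlap reverses the timeline on any tagged actor's exit, with no count of remaining occupants.
; RecordDeath is a stub that returns zero.
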(event `self.Box.OnComponentBeginOverlap`
  (params (OverlappedComponent :type "PrimitiveComponent Object Reference") (OtherActor :type "Actor Object Reference") (OtherComp :type "PrimitiveComponent Object Reference") (OtherBodyIndex :type Integer) (bFromSweep :type Boolean) (SweepResult :type "HitResult Structure (by ref)"))
  (if (or (`self.ActorHasTag` OtherActor "Player") (`self.ActorHasTag` OtherActor "AI"))
    (bind (_direction _alpha) (`Timeline|Open  Close Timeline` :!label _label)
      (:`Update`
        (`|ExecutionSequence`
          (:`then_0`
            (`SceneComponent.K2_SetRelativeLocation` (`self.Door1`) (`KismetMathLibrary.VLerp` (3.1e-05 46.884094 0.0) (3.1e-05 136.884094 0.0) _alpha) false false))
          (:`then_1`
            (`SceneComponent.K2_SetRelativeLocation` (`self.Door2`) (`KismetMathLibrary.VLerp` (-0.001007 -133.245789 0.0) (-0.001007 -233.245789 0.0) _alpha) false false)))))))

(event `self.Box.OnComponentEndOverlap`
  (params (OverlappedComponent :type "PrimitiveComponent Object Reference") (OtherActor :type "Actor Object Reference") (OtherComp :type "PrimitiveComponent Object Reference") (OtherBodyIndex :type Integer))
  (if (or (`self.ActorHasTag` OtherActor "Player") (`self.ActorHasTag` OtherActor "AI"))
    (goto _label :!via `Reverse`)))

(fn `Record Death`
  (returns (`Current Deaths` :type Integer))
  (return 0))

(fn `UserConstructionScript`)