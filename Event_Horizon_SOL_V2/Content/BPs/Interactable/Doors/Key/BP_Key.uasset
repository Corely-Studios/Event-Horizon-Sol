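; BP_Key is a key pickup, filed with the door interactables, that the player can carry in hand.
; A sphere overlap shows or hides its widget for actors tagged Player.
; Interact makes the player drop the current item, disables physics and collision, snaps the key to the hand socket and registers it as CurrentHeldItem.
; RecordDeath is a stub returning zero, and no unlocking logic lives here.
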(event `self.Sphere.OnComponentBeginOverlap`
  (params (OverlappedComponent :type "PrimitiveComponent Object Reference") (OtherActor :type "Actor Object Reference") (OtherComp :type "PrimitiveComponent Object Reference") (OtherBodyIndex :type Integer) (bFromSweep :type Boolean) (SweepResult :type "HitResult Structure (by ref)"))
  (if (`self.ActorHasTag` OtherActor "Player")
    (`SceneComponent.SetVisibility` (`self.Widget`) true false)))

(event `self.Sphere.OnComponentEndOverlap`
  (params (OverlappedComponent :type "PrimitiveComponent Object Reference") (OtherActor :type "Actor Object Reference") (OtherComp :type "PrimitiveComponent Object Reference") (OtherBodyIndex :type Integer))
  (if (`self.ActorHasTag` OtherActor "Player")
    (`SceneComponent.SetVisibility` (`self.Widget`) false false)))

(event `/Game/BPs/Interactable/Interface/BPI_Interaction.Interact`
  (params (`Player Ref` :type "/Game/BPs/Characters/FirstPersonBP/Blueprints/FirstPersonCharacter Object Reference"))
  (bind _object (`self.Object`))
  (`/Game/BPs/Characters/FirstPersonBP/Blueprints/FirstPersonCharacter.Drop Item` `Player Ref`)
  (`PrimitiveComponent.SetSimulatePhysics` _object false)
  (`PrimitiveComponent.SetCollisionEnabled` _object "NoCollision")
  (`self.K2_AttachToComponent` (`/Game/BPs/Characters/FirstPersonBP/Blueprints/FirstPersonCharacter.Hand Socket` `Player Ref`) "Hand Socket" "SnapToTarget" "SnapToTarget" "KeepWorld")
  (set `/Game/BPs/Characters/FirstPersonBP/Blueprints/FirstPersonCharacter.Current Held Item` self `Player Ref`))

(fn `Record Death`
  (returns (`Current Deaths` :type Integer))
  (return 0))

(fn `UserConstructionScript`)