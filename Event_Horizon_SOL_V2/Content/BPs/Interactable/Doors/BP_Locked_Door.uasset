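; Interactable locked door that unlocks and opens when the player's held item matches the RequiredKey class.
; A sphere overlap toggles the prompt widget for the player, and Interact flip-flops a timeline that swings the door open or closed.
; Without the key, Interact briefly shows a lock widget, guarded by a DoOnce against stacking.
; AI entering AIArea swing an unlocked door through a separate timeline, which reverses after a short delay.
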(event `self.Sphere.OnComponentBeginOverlap`
  (params (OverlappedComponent :type "PrimitiveComponent Object Reference") (OtherActor :type "Actor Object Reference") (OtherComp :type "PrimitiveComponent Object Reference") (OtherBodyIndex :type Integer) (bFromSweep :type Boolean) (SweepResult :type "HitResult Structure (by ref)"))
  (if (`self.ActorHasTag` OtherActor "Player")
    (`SceneComponent.SetVisibility` (`self.Widget`) true false)))

(event `self.Sphere.OnComponentEndOverlap`
  (params (OverlappedComponent :type "PrimitiveComponent Object Reference") (OtherActor :type "Actor Object Reference") (OtherComp :type "PrimitiveComponent Object Reference") (OtherBodyIndex :type Integer))
  (if (`self.ActorHasTag` OtherActor "Player")
    (`SceneComponent.SetVisibility` (`self.Widget`) false false)))

(event `/Game/BPs/Interactable/Interface/BPI_Interaction.Interact`
  (params (`Player Ref` :type "/Game/BPs/Characters/FirstPersonBP/Blueprints/FirstPersonCharacter Object Reference"))
  (if (`self.Is Unlocked?`)
    _
    (elif (== (`GameplayStatics.GetObjectClass` (`/Game/BPs/Characters/FirstPersonBP/Blueprints/FirstPersonCharacter.Current Held Item` `Player Ref`)) (`self.Required Key`))
      (set `self.Is Unlocked?` true)
      (else
        (`/Engine/EditorBlueprintResources/StandardMacros.DoOnce` false :!label _label
          (:`Completed`
            (bind _returnvalue (`|CreateWidget` "/Game/UI/Widgets/Puzzles/Key/WBP_Key_Lock.WBP_Key_Lock_C" (`GameplayStatics.GetPlayerController` 0)))
            (`UserWidget.AddToViewport` _returnvalue 0)
            (`KismetSystemLibrary.Delay` 2.0)
            (`Widget.RemoveFromParent` _returnvalue)
            (goto _label :!via `Reset`))))))
  (`/Engine/EditorBlueprintResources/StandardMacros.FlipFlop`
    (:`A`
      (bind (_direction _alpha) (`Timeline|Open Close Timeline` :!label _label_2)
        (:`Update`
          (`SceneComponent.K2_SetRelativeRotation` (`self.Door`) (`KismetMathLibrary.RLerp` (struct) (struct :`Yaw` -100.0) _alpha) false false))))
    (:`B`
      (goto _label_2 :!via `Reverse`))))

(event `self.AI Area.OnComponentBeginOverlap`
  (params (OverlappedComponent :type "PrimitiveComponent Object Reference") (OtherActor :type "Actor Object Reference") (OtherComp :type "PrimitiveComponent Object Reference") (OtherBodyIndex :type Integer) (bFromSweep :type Boolean) (SweepResult :type "HitResult Structure (by ref)"))
  (if (`self.ActorHasTag` OtherActor "AI")
    (if (`self.Is Unlocked?`)
      (`|ExecutionSequence`
        (:`then_0`
          (bind (_direction _alpha) (`Timeline|AI Door TM` :!label _label_3)
            (:`Update`
              (`SceneComponent.K2_SetRelativeRotation` (`self.Door`) (`KismetMathLibrary.RLerp` (struct) (struct :`Yaw` -100.0) _alpha) false false))))
        (:`then_1`
          (`KismetSystemLibrary.Delay` 0.5)
          (goto _label_3 :!via `Reverse`))))))

(fn `Record Death`
  (returns (`Current Deaths` :type Integer))
  (return 0))

(fn `UserConstructionScript`)