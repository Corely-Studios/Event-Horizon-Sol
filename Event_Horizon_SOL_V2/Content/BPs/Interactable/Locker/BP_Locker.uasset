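; BP_Locker is an interactable hiding locker that shows a widget while the player is inside its sphere.
; Interact toggles occupancy, the player's hiding state and capsule collision, with timelines swinging the door and lerping the player between hiding and exit spots.
; If the BP_AI can see the player hide, its blackboard records that and this locker as target.
; MonsterKillDoor swings the door and pulls the player out, restoring collision.
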(event `self.Sphere.OnComponentBeginOverlap`
  (params (OverlappedComponent :type "PrimitiveComponent Object Reference") (OtherActor :type "Actor Object Reference") (OtherComp :type "PrimitiveComponent Object Reference") (OtherBodyIndex :type Integer) (bFromSweep :type Boolean) (SweepResult :type "HitResult Structure (by ref)"))
  (if (`self.ActorHasTag` OtherActor "Player")
    (`SceneComponent.SetVisibility` (`self.Widget`) true false)))

(event `self.Sphere.OnComponentEndOverlap`
  (params (OverlappedComponent :type "PrimitiveComponent Object Reference") (OtherActor :type "Actor Object Reference") (OtherComp :type "PrimitiveComponent Object Reference") (OtherBodyIndex :type Integer))
  (if (`self.ActorHasTag` OtherActor "Player")
    (`SceneComponent.SetVisibility` (`self.Widget`) false false)))

(event `/Game/BPs/Interactable/Interface/BPI_Interaction.Interact`
  (params (`Player Ref` :type "/Game/BPs/Characters/FirstPersonBP/Blueprints/FirstPersonCharacter Object Reference"))
  (set `self.Player` `Player Ref`)
  (if (not (`self.Is Occupied?`))
    (set `self.Is Occupied?` true)
    (set `/Game/BPs/Characters/FirstPersonBP/Blueprints/FirstPersonCharacter.IsHiding?` true (`self.Player`))
    (`PrimitiveComponent.SetCollisionEnabled` (`Character.CapsuleComponent` (`self.Player`)) "NoCollision")
    (bind _returnvalue (`GameplayStatics.GetActorOfClass` "/Game/BPs/Characters/AI/BP_AI.BP_AI_C"))
    (`/Engine/EditorBlueprintResources/StandardMacros.IsValid` _returnvalue
      (:`Is Valid`
        (bind _returnvalue_2 (`AIBlueprintHelperLibrary.GetBlackboard` (`AIBlueprintHelperLibrary.GetAIController` _returnvalue)))
        (if (`BlackboardComponent.GetValueAsBool` _returnvalue_2 "Can See Player?")
          (`BlackboardComponent.SetValueAsBool` _returnvalue_2 "Saw Player Hide?" true)
          (`BlackboardComponent.SetValueAsObject` _returnvalue_2 "Target Locker" self)
          (bind (_direction _door_rotation) (`Timeline|Door Lerp` :!label _label)
            (:`Update`
              (`SceneComponent.K2_SetRelativeRotation` (`self.Locker Door`) (`KismetMathLibrary.RLerp` (struct) (struct :`Yaw` 90.0) _door_rotation) false false))
            (:`Finished`
              (`/Engine/EditorBlueprintResources/StandardMacros.DoOnce` false :!label _label_2
                (:`Completed`
                  (bind (_direction_2 _player_alpha) (`Timeline|Player Inside Lerp`)
                    (:`Update`
                      (`self.K2_SetActorRelativeLocation` (`self.Player`) (`KismetMathLibrary.VLerp` (`self.K2_GetActorLocation` (`self.Player`)) (`SceneComponent.K2_GetComponentLocation` (`self.Hiding Spot`)) _player_alpha) false false)
                      (goto _label :!via `Reverse`)))))))
          (else
            (`|ExecutionSequence` :!label _label_3
              (:`then_0`
                (goto _label))
              (:`then_1`
                (goto _label_5 :!via `Reset`))))))
      (:`Is Not Valid`
        (goto _label_3)))
    (else
      (set `self.Is Occupied?` false)
      (set `/Game/BPs/Characters/FirstPersonBP/Blueprints/FirstPersonCharacter.IsHiding?` false (`self.Player`))
      (`PrimitiveComponent.SetCollisionEnabled` (`Character.CapsuleComponent` (`self.Player`)) "QueryAndPhysics")
      (`|ExecutionSequence`
        (:`then_0`
          (bind (_direction_3 _door_rotation_2) (`Timeline|Door Lerp 2` :!label _label_4)
            (:`Update`
              (`SceneComponent.K2_SetRelativeRotation` (`self.Locker Door`) (`KismetMathLibrary.RLerp` (struct) (struct :`Yaw` 90.0) _door_rotation_2) false false))
            (:`Finished`
              (`/Engine/EditorBlueprintResources/StandardMacros.DoOnce` false :!label _label_5
                (:`Completed`
                  (bind (_direction_4 _player_alpha_2) (`Timeline|Player Exit Lerp`)
                    (:`Update`
                      (`self.K2_SetActorRelativeLocation` (`self.Player`) (`KismetMathLibrary.VLerp` (`self.K2_GetActorLocation` (`self.Player`)) (`SceneComponent.K2_GetComponentLocation` (`self.Exit Spot `)) _player_alpha_2) false false)
                      (goto _label_4 :!via `Reverse`))))))))
        (:`then_1`
          (goto _label_2 :!via `Reset`))))))

(event `/Game/BPs/Interactable/Interface/BPI_Interaction.Monster Kill Door`
  (bind (_direction _door_rotation) (`Timeline|Kill Door TM`)
    (:`Update`
      (`SceneComponent.K2_SetRelativeRotation` (`self.Locker Door`) (`KismetMathLibrary.RLerp` (struct) (struct :`Yaw` 90.0) _door_rotation) false false))
    (:`Finished`
      (`/Engine/EditorBlueprintResources/StandardMacros.DoOnce` false
        (:`Completed`
          (bind (_direction_2 _player_alpha) (`Timeline|Player Outside Kill TM`)
            (:`Update`
              (`self.K2_SetActorRelativeLocation` (`self.Player`) (`KismetMathLibrary.VLerp` (`SceneComponent.K2_GetComponentLocation` (`self.Hiding Spot`)) (+ (`self.K2_GetActorLocation` (`self.Player`)) (0.0 20.0 0.0)) _player_alpha) false false)
              (`PrimitiveComponent.SetCollisionEnabled` (`Character.CapsuleComponent` (`self.Player`)) "QueryAndPhysics"))))))))

(fn `Record Death`
  (returns (`Current Deaths` :type Integer))
  (return 0))

(fn `UserConstructionScript`)