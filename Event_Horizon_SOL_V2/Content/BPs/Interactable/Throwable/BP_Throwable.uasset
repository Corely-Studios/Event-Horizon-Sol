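; BP_Throwable is an interactable throwable object that shows a prompt widget while the player is inside its sphere.
; Interact passes the player reference to the parent implementation.
; Separate events create the WBP_Throwable viewport widget and remove it.
; When the object hits an actor tagged AI, it drops its own Flying tag.
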(event `self.Sphere.OnComponentBeginOverlap`
  (params (OverlappedComponent :type "PrimitiveComponent Object Reference") (OtherActor :type "Actor Object Reference") (OtherComp :type "PrimitiveComponent Object Reference") (OtherBodyIndex :type Integer) (bFromSweep :type Boolean) (SweepResult :type "HitResult Structure (by ref)"))
  (if (`self.ActorHasTag` OtherActor "Player")
    (`SceneComponent.SetVisibility` (`self.Widget`) true false)))

(event `self.Sphere.OnComponentEndOverlap`
  (params (OverlappedComponent :type "PrimitiveComponent Object Reference") (OtherActor :type "Actor Object Reference") (OtherComp :type "PrimitiveComponent Object Reference") (OtherBodyIndex :type Integer))
  (if (`self.ActorHasTag` OtherActor "Player")
    (`SceneComponent.SetVisibility` (`self.Widget`) false false)))

(event `/Game/BPs/Interactable/Interface/BPI_Interaction.Interact`
  (params (`Player Ref` :type "/Game/BPs/Characters/FirstPersonBP/Blueprints/FirstPersonCharacter Object Reference") (`Clicked Component` :type "PrimitiveComponent Object Reference"))
  (`parent.Interact` `Player Ref` null))

(event `/Game/BPs/Interactable/Interface/BPI_Interaction.Destroy My Widget`
  (`Widget.RemoveFromParent` (`self.ThrowWidget Ref`)))

(event `Initialize UI`
  (bind _returnvalue (`|CreateWidget` "/Game/UI/Widgets/WBP_Throwable.WBP_Throwable_C"))
  (bind _output_get (set `self.ThrowWidget Ref` _returnvalue))
  (`UserWidget.AddToViewport` _output_get 0))

(event `self.Object.OnComponentHit`
  (params (HitComponent :type "PrimitiveComponent Object Reference") (OtherActor :type "Actor Object Reference") (OtherComp :type "PrimitiveComponent Object Reference") (NormalImpulse :type "Vector Structure") (Hit :type "HitResult Structure (by ref)"))
  (if (`self.ActorHasTag` OtherActor "AI")
    (`KismetArrayLibrary.Array_RemoveItem` (`self.Tags`) "Flying")))

(fn `UserConstructionScript`)