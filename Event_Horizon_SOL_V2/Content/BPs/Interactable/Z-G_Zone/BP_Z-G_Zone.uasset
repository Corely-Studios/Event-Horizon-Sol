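; Zero-gravity zone volume that suspends gravity for the player and loose physics objects inside its Zone overlap component.
; On entry, actors tagged Player switch to Flying with zero gravity scale, and non-AI actors get gravity and linear damping turned off on their static mesh component.
; On exit, the player returns to Falling with normal gravity, and objects regain gravity and slight damping.
; Actors tagged AI are ignored.
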(event `self.Zone.OnComponentBeginOverlap`
  (params (OverlappedComponent :type "PrimitiveComponent Object Reference") (OtherActor :type "Actor Object Reference") (OtherComp :type "PrimitiveComponent Object Reference") (OtherBodyIndex :type Integer) (bFromSweep :type Boolean) (SweepResult :type "HitResult Structure (by ref)"))
  (bind _returnvalue (`self.GetComponentByClass` OtherActor "/Script/Engine.CharacterMovementComponent"))
  (bind _returnvalue_2 (`self.GetComponentByClass` OtherActor "/Script/Engine.StaticMeshComponent"))
  (if (`self.ActorHasTag` OtherActor "Player")
    (set `CharacterMovementComponent.GravityScale` 0.0 _returnvalue)
    (`CharacterMovementComponent.SetMovementMode` _returnvalue "MOVE_Flying" 0)
    (elif (not (`self.ActorHasTag` OtherActor "AI"))
      (`PrimitiveComponent.SetEnableGravity` _returnvalue_2 false)
      (`PrimitiveComponent.SetLinearDamping` _returnvalue_2 0.0))))

(event `self.Zone.OnComponentEndOverlap`
  (params (OverlappedComponent :type "PrimitiveComponent Object Reference") (OtherActor :type "Actor Object Reference") (OtherComp :type "PrimitiveComponent Object Reference") (OtherBodyIndex :type Integer))
  (bind _returnvalue (`self.GetComponentByClass` OtherActor "/Script/Engine.CharacterMovementComponent"))
  (bind _returnvalue_2 (`self.GetComponentByClass` OtherActor "/Script/Engine.StaticMeshComponent"))
  (if (`self.ActorHasTag` OtherActor "Player")
    (set `CharacterMovementComponent.GravityScale` 1.0 _returnvalue)
    (`CharacterMovementComponent.SetMovementMode` _returnvalue "MOVE_Falling" 0)
    (elif (not (`self.ActorHasTag` OtherActor "AI"))
      (`PrimitiveComponent.SetEnableGravity` _returnvalue_2 true)
      (`PrimitiveComponent.SetLinearDamping` _returnvalue_2 0.01))))

(fn `UserConstructionScript`)