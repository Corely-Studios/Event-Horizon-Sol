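; Enemy AI character that triggers a jumpscare message on Player-tagged actors entering its KillZone.
; A looping stuck check teleports it to a nearby reachable point if it has barely moved and cannot see the player.
; A director timer counts unseen time, then writes a point near the player to the blackboard's NoiseLocation, throttled by a resetting DoOnce.
; Capsule hits from Flying-tagged actors temporarily zero its walk speed, stunning it.
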(event `self.Kill Zone.OnComponentBeginOverlap`
  (params (OverlappedComponent :type "PrimitiveComponent Object Reference") (OtherActor :type "Actor Object Reference") (OtherComp :type "PrimitiveComponent Object Reference") (OtherBodyIndex :type Integer) (bFromSweep :type Boolean) (SweepResult :type "HitResult Structure (by ref)"))
  ;[1 1 1] Jumpscare
  (if (`self.ActorHasTag` OtherActor "Player")
    (message `/Game/BPs/Interactable/Interface/BPI_Interaction.Trigger Jumpscare` OtherActor self)))

(event `self.ReceiveBeginPlay`
  (`|ExecutionSequence`
    (:`then_0`
      (`KismetSystemLibrary.K2_SetTimerDelegate` (delegate `Check If Stuck`) 7.0 true))
    (:`then_1`
      (`KismetSystemLibrary.K2_SetTimerDelegate` (delegate `Director Tick`) 1.0 true))))

(event `Check If Stuck`
  (bind _returnvalue (`self.K2_GetActorLocation`))
  (if (< (`KismetMathLibrary.Vector_Distance` (`self.Previous Location`) _returnvalue) 50.0)
    (if (not (`BlackboardComponent.GetValueAsBool` (`AIBlueprintHelperLibrary.GetBlackboard` (`AIBlueprintHelperLibrary.GetAIController` self)) "Can See Player?"))
      (`self.K2_SetActorLocation` (`NavigationSystemV1.K2_GetRandomReachablePointInRadius` _returnvalue 400.0 null null) false true))
    (else
      (set `self.Previous Location` _returnvalue))))

(event `Director Tick`
  (bind _time_unseen (`self.Time Unseen`))
  (if (`BlackboardComponent.GetValueAsBool` (`AIBlueprintHelperLibrary.GetBlackboard` (`AIBlueprintHelperLibrary.GetAIController` self)) "Can See Player?")
    (set `self.Time Unseen` 0)
    (else
      (bind _output_get (set `self.Time Unseen` (+ _time_unseen 1)))
      (`KismetSystemLibrary.PrintString` (`KismetStringLibrary.Conv_IntToString` _output_get))
      (if (>= _time_unseen 10)
        (`/Engine/EditorBlueprintResources/StandardMacros.DoOnce` false :!label _label
          (:`Completed`
            (`BlackboardComponent.SetValueAsVector` (`AIBlueprintHelperLibrary.GetBlackboard` (`AIBlueprintHelperLibrary.GetAIController` self)) "NoiseLocation" (`NavigationSystemV1.K2_GetRandomReachablePointInRadius` (`self.K2_GetActorLocation` (`GameplayStatics.GetPlayerCharacter` 0)) 500.0 null null))
            (`KismetSystemLibrary.Delay` 30.0)
            (goto _label :!via `Reset`)))))))

(event `self.CapsuleComponent.OnComponentHit`
  (params (HitComponent :type "PrimitiveComponent Object Reference") (OtherActor :type "Actor Object Reference") (OtherComp :type "PrimitiveComponent Object Reference") (NormalImpulse :type "Vector Structure") (Hit :type "HitResult Structure (by ref)"))
  (bind _charactermovement (`self.CharacterMovement`))
  (if (`self.ActorHasTag` OtherActor "Flying")
    (set `CharacterMovementComponent.MaxWalkSpeed` 0.0 _charactermovement)
    (`KismetSystemLibrary.Delay` 5.0)
    (set `CharacterMovementComponent.MaxWalkSpeed` 300.0 _charactermovement)))

(fn `UserConstructionScript`)